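; Goal actor that bobs up and down in the level; the file holds no scoring or overlap logic.
; It stores its spawn location on BeginPlay, then each Tick sets its Z to that start height plus a sine of game time, scaled by period multiplier and amplitude variables.
; X and Y keep their current values, and the move does not sweep for collisions.
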(event `self.ReceiveBeginPlay`
  (set `self.StartPos` (`self.K2_GetActorLocation`)))

(event `self.ReceiveTick`
  (params (DeltaSeconds :type "Float (single-precision)"))
  (bind (_returnvalue_x _returnvalue_y) (`KismetMathLibrary.BreakVector` (`self.K2_GetActorLocation`)))
  (bind (_startpos_x _startpos_y _startpos_z) (`KismetMathLibrary.BreakVector` (`self.StartPos`)))
  (`self.K2_SetActorLocation` (`KismetMathLibrary.MakeVector` _returnvalue_x _returnvalue_y (+ _startpos_z (* (`KismetMathLibrary.Sin` (* (`GameplayStatics.GetTimeSeconds`) (`self.PeriodMultiplier`))) (`self.Amplitude`))))))

(fn `UserConstructionScript`)