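; First-person horror player character that carries a torch which burns out over a set lifetime.
; Tick shrinks the torch's attenuation radius by game time over Lifetime; near darkness it fires TorchOut, marks the player dead and shows the cursor.
; Axis inputs drive movement and look, with forward/back input scaling a horror camera shake.
; Overlapping a Goal fires GoalTouched and shows the cursor.
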(event `self.ReceiveBeginPlay`
  (set `self.TorchStartRadius` (`PointLightComponent.AttenuationRadius` (`self.Torch`))))

(event `self.ReceiveTick`
  (params (DeltaSeconds :type "Float (single-precision)"))
  (bind _returnvalue (`KismetMathLibrary.Lerp` (`self.TorchStartRadius`) 0.0 (/ (`GameplayStatics.GetTimeSeconds`) (`self.Lifetime`))))
  (if (not (`self.dead`))
    (`PointLightComponent.SetAttenuationRadius` (`self.Torch`) _returnvalue)
    (if (<= _returnvalue 100.0)
      (`self.TorchOut`)
      (set `self.dead` true)
      (set `PlayerController.bShowMouseCursor` true (`GameplayStatics.GetPlayerController` 0)))))

(event `InputAxis|Horizontal`
  (params (AxisValue :type "Float (single-precision)"))
  (`self.AddMovementInput` (`self.GetActorRightVector`) AxisValue))

(event `InputAxis|Vertical`
  (params (AxisValue :type "Float (single-precision)"))
  (`self.AddMovementInput` (`self.GetActorForwardVector`) AxisValue)
  (`PlayerController.ClientStartCameraShake` :`self` (`GameplayStatics.GetPlayerController` 0) :`Shake` "/Game/Blueprints/HorrorCameraShake.HorrorCameraShake_C" :`Scale` AxisValue))

(event `InputAxis|Azimuth`
  (params (AxisValue :type "Float (single-precision)"))
  (`self.AddControllerYawInput` AxisValue))

(event `InputAxis|Altitude`
  (params (AxisValue :type "Float (single-precision)"))
  (`self.AddControllerPitchInput` AxisValue))

(event `self.ReceiveActorBeginOverlap`
  (params (OtherActor :type "Actor Object Reference"))
  (cast `/Game/Blueprints/Goal` OtherActor)
  (`self.GoalTouched`)
  (set `PlayerController.bShowMouseCursor` true (`GameplayStatics.GetPlayerController` 0)))

(fn `UserConstructionScript`)